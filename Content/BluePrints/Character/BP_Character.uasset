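; Player character Blueprint with Enhanced Input movement, camera look and montage-based melee attacks using a collected weapon.
; A Locomotion/Battle state gates attacks: the first press plays AM_Attack, later presses set NextCombo from the current section, and AttackEnd restores Locomotion.
; Weapon pickup attaches the actor to the mesh socket and binds the attack-check dispatchers, so OnAttackCheckBegin/End calls reach the weapon's hit check.
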(event Custom|AttackEnd
  (Variables|Default|SetState_BP "NewEnumerator0"))

(event Custom|OnWeaponCollected
  (params (WeaponActor :type BP%20Weapon%20Object%20Reference))
  ;[0.15 0.15 0.15 0.5] 무기 습득 처리\
  (Actor|SetOwner WeaponActor self)
  (Transformation|AttachComponentToComponent WeaponActor (Variables|Character|GetMesh) "WeaponPosition" "SnapToTarget" "SnapToTarget" "SnapToTarget" true)
  (Variables|Default|SetWeaponActor WeaponActor)
  (Variables|Default|SetHasWeapon true)
  ;[0.15 0.15 0.15 0.5] 공격 판정 시작 이벤트에 함수 등록
  (EventDispatchers|BindEventtoAttackCheckBeginEvent (delegate Custom|RaiseAttackCheckBegin))
  ;[0.15 0.15 0.15 0.5] 공격 판정 종료 이벤트에 함수 등록
  (EventDispatchers|BindEventtoAttackCheckEndEvent (delegate Custom|RaiseAttackCheckEnd)))

(event Custom|OnAttackCheckBegin
  ;[0.15 0.15 0.15 0.5] 공격 판정 시작
  (Default|CallAttackCheckBeginEvent))

(event Custom|OnAttackCheckEnd
  ;[0.15 0.15 0.15 0.5] 공격 판정 종료
  (Default|CallAttackCheckEndEvent))

(event Custom|RaiseAttackCheckEnd
  ;[0.15 0.15 0.15 0.5] 공격 판정 종료 이벤트에 함수 등록
  (Utilities|IsValid (Variables|Default|GetWeaponActor)
    (:Is%20Valid
      (Default|OnAttackCheckEnd (Variables|Default|GetWeaponActor)))))

(event Custom|RaiseAttackCheckBegin
  ;[0.15 0.15 0.15 0.5] 공격 판정 시작 이벤트에 함수 등록
  (Utilities|IsValid (Variables|Default|GetWeaponActor)
    (:Is%20Valid
      (Default|OnAttackCheckBegin (Variables|Default|GetWeaponActor)))))

(event Input|EnhancedActionEvents|EnhancedInputActionIA_Move
  (params (ActionValue :type Vector%202D%20Structure) (ElapsedSeconds :type Float%20%28double-precision%29) (TriggeredSeconds :type Float%20%28double-precision%29) (InputAction :type Input%20Action%20Object%20Reference :default "/Game/BluePrints/Input/Actions/IA_Move.IA_Move"))
  ;[0.15 0.15 0.15 0.5] 이동
  (Pawn|Input|AddMovementInput (Math|Vector|GetRightVector (Pawn|GetControlRotation :!class /Script/Engine.Pawn)) (.x ActionValue) false)
  (Pawn|Input|AddMovementInput (Math|Vector|GetForwardVector (Math|Rotator|MakeRotator 0.0 0.0 (.yaw (Pawn|GetControlRotation :!class /Script/Engine.Pawn)))) (.y ActionValue) false))

(event Input|EnhancedActionEvents|EnhancedInputActionIA_View
  (params (ActionValue :type Vector%202D%20Structure) (ElapsedSeconds :type Float%20%28double-precision%29) (TriggeredSeconds :type Float%20%28double-precision%29) (InputAction :type Input%20Action%20Object%20Reference :default "/Game/BluePrints/Input/Actions/IA_View.IA_View"))
  ;[0.15 0.15 0.15 0.5] 카메라 회전
  (Pawn|Input|AddControllerYawInput (.x ActionValue)) ; 컨트롤러의 (Yaw)회전 추가
  (Pawn|Input|AddControllerPitchInput (* (.y ActionValue) -1.0)) ; 컨트롤러의 (Pitch)회전 추가
)

(event Input|EnhancedActionEvents|EnhancedInputActionIA_Attack
  (params (ActionValue :type Boolean) (ElapsedSeconds :type Float%20%28double-precision%29) (TriggeredSeconds :type Float%20%28double-precision%29) (InputAction :type Input%20Action%20Object%20Reference :default "/Game/BluePrints/Input/Actions/IA_Attack.IA_Attack"))
  ;[0.15 0.15 0.15 0.5] 공격
  (if (Variables|Default|GetHasWeapon)
    (switch Utilities|FlowControl|Switch|SwitchonBP_EPlayerState (Variables|Default|GetState_BP)
      (:NewEnumerator0
        (Variables|Default|SetState_BP "NewEnumerator1")
        (Animation|PlayAnimMontage "/Game/BluePrints/Character/AM_Attack.AM_Attack" 1.0 "None"))
      (:NewEnumerator1
        (switch name (Animation|Montage|MontageGetCurrentSection (Components|SkeletalMesh|GetAnimInstance (Variables|Character|GetMesh)) "/Game/BluePrints/Character/AM_Attack.AM_Attack")
          (:Attack1
            (Variables|Default|SetNextCombo "Attack2"))
          (:Attack2
            (Variables|Default|SetNextCombo "Attack3"))
          (:Attack3
            (Variables|Default|SetNextCombo "Attack4")))))))

(fn ConstructionScript)